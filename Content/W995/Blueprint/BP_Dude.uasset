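; BP_Dude is the 2D side-scrolling player character, with flipbook animation, running, jumping, climbing and shooting.
; Input drives a State value that UpdateAnimation maps to flipbooks, while climbing switches movement to Flying.
; Damage applies knockback, sprite blinking and an input lockout, or death at zero health.
; It also creates the HUD, spawns fire or ice shots from an arm arrow, and tracks experience-based levels.
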(event Custom|DamageSystem
  (params (DamageIn :type Float%20%28single-precision%29))
  ;[1 1 1] DamageSystem
  (Audio|PlaySound2D "/Game/W995/Sounds/player_damaged_Cue.player_damaged_Cue")
  (Input|DisableInput (Game|GetPlayerController 0))
  (Variables|Default|SetisHit true)
  (bind _output_get (Variables|Default|Sethealth_current (- (Variables|Default|Gethealth_current) DamageIn)))
  (if (<= _output_get 0.0)
    (Variables|Default|SetState "NewEnumerator5")
    (Input|DisableInput (Game|GetPlayerController 0))
    (CallFunction|UpdateAnimation)
    (Audio|PlaySound2D "/Game/W995/Sounds/player_dead_Cue.player_dead_Cue")
    (else
      (Variables|Default|SetState "NewEnumerator4")
      (CallFunction|UpdateAnimation)
      (Components|Movement|StopMovementImmediately (Variables|Character|GetCharacterMovement))
      (Physics|AddImpulse (Variables|Character|GetCharacterMovement) (Math|Vector|MakeVector (* (Variables|Default|GetFacing) (Variables|Default|GetKnockback)) 0.0 4e+04) false)
      (Utilities|Time|SetTimerbyFunctionName 0 "Blink" 0.1 true)
      (Utilities|FlowControl|Delay 2.0)
      (Utilities|Time|ClearTimerbyFunctionName 0 "Blink")
      (Rendering|SetVisibility (Variables|Default|GetSprite) true true)
      (Input|EnableInput (Game|GetPlayerController 0)))))

(event Custom|UpdateAnimation
  ;[1 1 1] Handle Animation
  (switch Utilities|FlowControl|Switch|SwitchonCharacterState (Variables|Default|GetState)
    (:NewEnumerator0
      (Sprite|SetFlipbook (Variables|Default|GetSprite) (select (Utilities|IsMovingMacro) "/Game/W995/Sprites/Character/A_Run.A_Run" "/Game/W995/Sprites/Character/A_Idle.A_Idle")))
    (:NewEnumerator2
      (Sprite|SetFlipbook (Variables|Default|GetSprite) "/Game/W995/Sprites/Character/A_Jump.A_Jump"))
    (:NewEnumerator4
      (Sprite|SetFlipbook (Variables|Default|GetSprite) "/Game/W995/Sprites/Character/A_Hit.A_Hit"))
    (:NewEnumerator5
      (Sprite|SetFlipbook (Variables|Default|GetSprite) "/Game/W995/Sprites/Character/A_Dead.A_Dead"))
    (:NewEnumerator6
      (Sprite|SetFlipbook (Variables|Default|GetSprite) "/Game/W995/Sprites/Character/A_Sitting.A_Sitting"))
    (:NewEnumerator7
      (if (Variables|Default|GetisJumping)
        (Sprite|SetFlipbook (Variables|Default|GetSprite) "/Game/W995/Sprites/Character/A_JumpShoot.A_JumpShoot")
        (elif (Variables|Default|GetisClimbing)
          (Sprite|SetFlipbook (Variables|Default|GetSprite) "/Game/W995/Sprites/Character/A_ClimbShoot.A_ClimbShoot")
          (elif (Utilities|IsMovingMacro)
            (Sprite|SetFlipbook (Variables|Default|GetSprite) "/Game/W995/Sprites/Character/A_RunShoot.A_RunShoot")
            (else
              (Sprite|SetFlipbook (Variables|Default|GetSprite) "/Game/W995/Sprites/Character/A_Shoot.A_Shoot"))))))
    (:NewEnumerator8
      (Sprite|SetFlipbook (Variables|Default|GetSprite) "/Game/W995/Sprites/Character/A_Climb.A_Climb"))))

(event Custom|Blink
  ;[1 1 1] DamageSystem
  (Rendering|ToggleVisibility (Variables|Default|GetSprite) true))

(event Custom|GainHealth
  (params (HealthToAdd :type Float%20%28single-precision%29))
  ;[1 1 1] Gain Health
  (Variables|Default|Sethealth_current (Math|Float|Clamp(Float) (+ (Variables|Default|Gethealth_current) HealthToAdd))))

(event Custom|GainExperience
  (params (ExperienceToGain :type Integer))
  ;[1 1 1] GainExperience
  (bind _level (CallFunction|GetLevelforExperience (Variables|Stats|GetCurrentExperience)))
  (if (<= _level (Variables|Stats|GetCurrentLevel))
    (Development|PrintString "True")
    (else
      (Development|PrintString "LEVEL UP!!!!")))
  (bind _output_get (Variables|Stats|SetCurrentExperience (+ ExperienceToGain (Variables|Stats|GetCurrentExperience))))
  (bind _level_2 (CallFunction|GetLevelforExperience _output_get))
  (Variables|Stats|SetCurrentLevel _level_2))

(event EventOnLanded
  (params (Hit :type Hit%20Result%20Structure%20%28by%20ref%29))
  ;[1 1 1] Landing / post damange
  (Variables|Default|SetisJumping false)
  (if (Variables|Default|GetisHit)
    (Variables|Default|SetState "NewEnumerator6")
    (CallFunction|UpdateAnimation)
    (Utilities|FlowControl|Delay 0.5)
    (Variables|Default|SetisHit false)
    (Variables|Default|SetState "NewEnumerator0")
    (CallFunction|UpdateAnimation)
    (Input|EnableInput (Game|GetPlayerController 0))
    (else
      (Variables|Default|SetState "NewEnumerator0")
      (CallFunction|UpdateAnimation))))

(event EventBeginPlay
  ;[0.9855 0.3735 1] Init
  (Utilities|FlowControl|Sequence
    (:then_0
      (Class|ActorComponent|SetIsReplicated (Variables|Default|GetSprite) true))
    (:then_1
      (bind _returnvalue (UserInterface|CreateWidget "/Game/W995/Blueprint/Widget_HUD.Widget_HUD_C" (Game|GetPlayerController 0)))
      (bind _output_get (Variables|Default|SetHealthBar _returnvalue))
      (UserInterface|Viewport|AddtoViewport _output_get 0))))

(event Input|ActionEvents|InputActionShoot
  ;[1 1 1] Shoot
  (:Pressed
    (CallFunction|FireSelectedWeapon)
    (Variables|Default|SetState "NewEnumerator7")
    (Audio|PlaySound2D "/Game/W995/Sounds/player_shot_Cue.player_shot_Cue")
    (CallFunction|UpdateAnimation :!label _label))
  (:Released
    (Utilities|FlowControl|RetriggerableDelay 0.2)
    (CallFunction|RestoretoIdle)
    (goto _label)))

(event Input|ActionEvents|InputActionJump
  ;[1 1 1] Handle Jump
  (:Pressed
    (CallFunction|StopClimb)
    (Character|Jump)
    (if (not (Variables|Default|GetisJumping))
      (Audio|PlaySound2D "/Game/W995/Sounds/player_jump_Cue.player_jump_Cue")
      (Variables|Default|SetState "NewEnumerator2")
      (Variables|Default|SetisJumping true)))
  (:Released
    (Character|StopJumping)))

(event Input|AxisEvents|InputAxisMoveUp
  (params (AxisValue :type Float%20%28single-precision%29))
  (bind _returnvalue (== AxisValue 0.0))
  ;[1 1 1] Climb
  (if (Variables|Default|GetcanClimb)
    (if (Variables|Default|GetisClimbing)
      (if _returnvalue
        (Variables|/Script/Engine.MovementComponent|SetVelocity (Variables|Character|GetCharacterMovement) "0, 0, 0")
        (Components|Timeline|SetPlayRate (Variables|Default|GetSprite) 0.0)
        (else
          (Pawn|Input|AddMovementInput "0.000000, 0,10.000000" AxisValue true :!label _label)
          (Components|Timeline|SetPlayRate (Variables|Default|GetSprite) 1.0)))
      (elif (not _returnvalue)
        (CallFunction|StartClimb)
        (goto _label)))))

(event Input|AxisEvents|InputAxisMoveRight
  (params (AxisValue :type Float%20%28single-precision%29))
  ;[1 1 1] Handle movement
  (if (not (Variables|Default|GetisClimbing))
    (Pawn|Input|AddMovementInput "1.000000, 0, 0" AxisValue false)
    (CallFunction|UpdateAnimation)
    (Math|Float|CompareFloat AxisValue 0.0
      (:>
        (Pawn|SetControlRotation (Pawn|GetController) (Class|KismetMathLibrary|MakeRot 0.0 0.0 0.0))
        (Variables|Default|SetFacing 1))
      (:<
        (Pawn|SetControlRotation (Pawn|GetController) (Class|KismetMathLibrary|MakeRot 0.0 1.8e+02 0.0))
        (Variables|Default|SetFacing -1)))))

(event Input|KeyboardEvents|1
  ;[1 1 1] ChangeWeapon
  (:Pressed
    (Variables|Default|SetCurrentWeapon "/Game/W995/Blueprint/Weapons/BP_Shot_Fire.BP_Shot_Fire_C")))

(event Input|KeyboardEvents|2
  ;[1 1 1] ChangeWeapon
  (:Pressed
    (Variables|Default|SetCurrentWeapon "/Game/W995/Blueprint/Weapons/BP_Shot_Ice.BP_Shot_Ice_C")))

(event Input|TouchEvents|InputTouch
  (params (Location :type Vector) (FingerIndex :type ETouchIndex%20Enum))
  ;[1 1 1] Handle Jump
  (:Pressed
    (Character|Jump)
    (if (not (Variables|Default|GetisJumping))
      (Audio|PlaySound2D "/Game/W995/Sounds/player_jump_Cue.player_jump_Cue")
      (Variables|Default|SetState "NewEnumerator2")
      (Variables|Default|SetisJumping true)))
  (:Released
    (Character|StopJumping)))

(fn ConstructionScript)

(fn IsMoving
  (return (> (Math|Vector|VectorLength (Transformation|GetVelocity)) 0.0)))

(fn GetLevelforExperience
  (params (ExperienceToCheck :type Integer))
  (return (Math|Float|Floor (/ (Math|Conversions|ToFloat(Integer) (Variables|Stats|GetCurrentExperience)) 1.5e+02))))

(fn FireSelectedWeapon
  (Game|SpawnActorfromClass (Variables|Default|GetCurrentWeapon) (Transformation|GetWorldTransform (Variables|Default|GetArrowShotArm)) false 0 0)
  (return 0))

(fn StartClimb
  (Variables|Default|SetisClimbing true)
  (Pawn|Components|CharacterMovement|SetMovementMode (Variables|Character|GetCharacterMovement) "MOVE_Flying" 0)
  (Variables|Default|SetState "NewEnumerator8")
  (CallFunction|UpdateAnimation))

(fn StopClimb
  (if (Variables|Default|GetisClimbing)
    (Variables|Default|SetisClimbing false)
    (Variables|Default|SetState "NewEnumerator0")
    (Pawn|Components|CharacterMovement|SetMovementMode (Variables|Character|GetCharacterMovement) "MOVE_Walking" 0)
    (CallFunction|UpdateAnimation)))

(fn RestoretoIdle
  (if (Variables|Default|GetisClimbing)
    (Variables|Default|SetState "NewEnumerator8")
    (else
      (Variables|Default|SetState "NewEnumerator0"))))