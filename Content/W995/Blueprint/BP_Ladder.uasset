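; BP_Ladder is a placeable 2D sprite ladder that lets BP_Dude climb while overlapping it.
; Its construction script uses the length of EndLocation to stack collision-free ladder sprites upward at 16-unit intervals and resize the narrow Box extent to match.
; Overlap begin sets the dude's CanClimb flag, while overlap end clears it and calls StopClimb.
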(event EventBeginPlay)

(event Collision|EventActorBeginOverlap
  (params (OtherActor :type Actor%20Object%20Reference))
  (bind _asbp_dude (Utilities|Casting|CastToBP_Dude OtherActor))
  (Variables|/Game/W995/Blueprint/BP_Dude.BP_Dude_C|SetcanClimb _asbp_dude true))

(event EventTick
  (params (DeltaSeconds :type Float%20%28single-precision%29)))

(event Collision|EventActorEndOverlap
  (params (OtherActor :type Actor%20Object%20Reference))
  (bind _asbp_dude (Utilities|Casting|CastToBP_Dude OtherActor))
  (Variables|/Game/W995/Blueprint/BP_Dude.BP_Dude_C|SetcanClimb _asbp_dude false)
  (Default|StopClimb _asbp_dude))

(fn ConstructionScript
  (bind _endlocation (Variables|Default|GetEndLocation))
  (bind _returnvalue (Math|Vector|VectorLength _endlocation))
  (if (Math|Vector|NotEqual(Vector) (Variables|Default|GetEndLocation) "0, 0, 0" 0.0001)
    (for _index (range 1 (Math|Float|Floor (/ _returnvalue 16.0)))
      (bind _returnvalue_2 (AddComponent|AddPaperSpriteComponent false))
      (Collision|SetCollisionEnabled _returnvalue_2 "NoCollision")
      (Rendering|Components|Sprite|SetSprite _returnvalue_2 "/Game/W995/Sprites/Env/s_ladder.s_ladder")
      (Class|SceneComponent|Attachto _returnvalue_2 (Variables|Default|GetLadderSprite) "None" "KeepWorldPosition" true)
      (Transformation|SetRelativeLocation _returnvalue_2 (Math|Vector|MakeVector 0.0 0.0 (* _index 16.0)) false))
    (Components|Box|SetBoxExtent (Variables|Default|GetBox) (Math|Vector|MakeVector 2.0 0.0 _returnvalue) true)))