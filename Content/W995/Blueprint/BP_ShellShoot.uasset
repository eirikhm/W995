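; BP_ShellShoot is a sprite-based shell hazard that opens when BP_Dude comes near and hurts it on contact.
; Overlapping BoxPlayerCollide calls the player's DamageSystem with a small fixed amount.
; Entering or leaving ShootRangeBox swaps the open and closed sprites, snapping the sprite's yaw to the player-to-shell direction only at those moments.
; Despite the name, the graph contains no firing logic.
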(event OnComponentBeginOverlap(BoxPlayerCollide)
  (params (OtherActor :type Actor%20Object%20Reference) (OtherComp :type Primitive%20Component%20Object%20Reference) (OtherBodyIndex :type Integer) (bFromSweep :type Boolean) (SweepResult :type Hit%20Result%20Structure%20%28by%20ref%29))
  ;[1 1 1] Hurt player on contact
  (bind _asbp_dude (Utilities|Casting|CastToBP_Dude OtherActor))
  (Default|DamageSystem _asbp_dude 0.1))

(event OnComponentBeginOverlap(ShootRangeBox)
  (params (OtherActor :type Actor%20Object%20Reference) (OtherComp :type Primitive%20Component%20Object%20Reference) (OtherBodyIndex :type Integer) (bFromSweep :type Boolean) (SweepResult :type Hit%20Result%20Structure%20%28by%20ref%29))
  ;[1 1 1] Open shell
  (Utilities|Casting|CastToBP_Dude OtherActor)
  (Rendering|Components|Sprite|SetSprite (Variables|Default|GetShellSprite) "/Game/W995/Sprites/Enemies/shell_02.shell_02")
  (Transformation|SetWorldRotation (Variables|Default|GetShellSprite) (Class|KismetMathLibrary|MakeRot 0.0 (.Yaw (Class|KismetMathLibrary|BreakRot (Math|Conversions|RotationFromXVector (Math|Vector|GetForwardVector (Math|Rotator|FindLookatRotation (Transformation|GetActorLocation (Game|GetPlayerCharacter 0)) (Transformation|GetActorLocation)))))) 0.0) false))

(event OnComponentEndOverlap(ShootRangeBox)
  (params (OtherActor :type Actor%20Object%20Reference) (OtherComp :type Primitive%20Component%20Object%20Reference) (OtherBodyIndex :type Integer))
  ;[1 1 1] Close shell
  (Utilities|Casting|CastToBP_Dude OtherActor)
  (Rendering|Components|Sprite|SetSprite (Variables|Default|GetShellSprite) "/Game/W995/Sprites/Enemies/shell_01.shell_01")
  (Transformation|SetWorldRotation (Variables|Default|GetShellSprite) (Class|KismetMathLibrary|MakeRot 0.0 (.Yaw (Class|KismetMathLibrary|BreakRot (Math|Conversions|RotationFromXVector (Math|Vector|GetForwardVector (Math|Rotator|FindLookatRotation (Transformation|GetActorLocation (Game|GetPlayerCharacter 0)) (Transformation|GetActorLocation)))))) 0.0) false))

(fn ConstructionScript)