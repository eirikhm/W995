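; Base enemy Actor that takes damage, hurts the player on contact and awards experience when killed.
; DamageSystem subtracts health; at zero it destroys the actor, plays an explosion sound and grants experience to BP_Dude.
; Surviving hits trigger a short looping-timer blink that toggles HitPlayerBox and its children's visibility, then restores it.
; HitPlayerBox overlaps call BP_Dude's own DamageSystem with the contact damage value.
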(event OnComponentBeginOverlap(HitPlayerBox)
  (params (OtherActor :type Actor%20Object%20Reference) (OtherComp :type Primitive%20Component%20Object%20Reference) (OtherBodyIndex :type Integer) (bFromSweep :type Boolean) (SweepResult :type Hit%20Result%20Structure%20%28by%20ref%29))
  ;[1 1 1] Hurt Player
  (bind _asbp_dude (Utilities|Casting|CastToBP_Dude OtherActor))
  (Default|DamageSystem _asbp_dude (Variables|Default|GetPlayerHurtOnHit)))

(event Custom|DamageSystem
  (params (DamageToTake :type Float%20%28single-precision%29))
  ;[1 1 1] DamageSystem
  (bind _output_get (Variables|Default|SetCurrentHealth (- (Variables|Default|GetCurrentHealth) DamageToTake)))
  (if (<= _output_get 0.0)
    (Actor|DestroyActor)
    (Audio|PlaySound2D "/Game/W995/Sounds/explode_Cue.explode_Cue")
    (bind _asbp_dude (Utilities|Casting|CastToBP_Dude (Game|Player|GetPlayerPawn 0)))
    (Default|GainExperience _asbp_dude (Variables|Default|GetBaseExperienceValue))
    (else
      (Utilities|Time|SetTimerbyFunctionName 0 "Blink" 0.1 true)
      (Utilities|FlowControl|Delay 1.5)
      (Utilities|Time|ClearTimerbyFunctionName 0 "Blink")
      (Rendering|SetVisibility (Variables|Default|GetHitPlayerBox) true true))))

(event Custom|Blink
  ;[1 1 1] DamageSystem
  (Rendering|ToggleVisibility (Variables|Default|GetHitPlayerBox) true))

(event EventBeginPlay)

(event Collision|EventActorBeginOverlap
  (params (OtherActor :type Actor%20Object%20Reference)))

(event EventTick
  (params (DeltaSeconds :type Float%20%28single-precision%29)))

(fn ConstructionScript)