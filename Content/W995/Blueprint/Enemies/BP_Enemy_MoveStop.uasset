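; Moving enemy Blueprint whose HitPlayerBox shuttles between its relative origin and EndLocation, pausing at each end.
; Forward and Rewind play MoveStopTimeline in alternating directions, lerping the box and waiting StopDelay before reversing.
; BeginPlay only calls the parent and nothing here starts the loop; the TravelTime play-rate setup is unconnected.
; The construction script sets the whole actor's location to EndLocation or world origin, depending on TestEndLocation.
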(event Custom|Forward
  (bind (_direction _lerp_alpha) (Timeline|MoveStopTimeline PlayFromStart)
    (:Update
      (Transformation|SetRelativeLocation (Variables|Default|GetHitPlayerBox) (Math|Vector|Lerp(Vector) "0, 0, 0" (Variables|Default|GetEndLocation) _lerp_alpha) false))
    (:Finished
      (Utilities|FlowControl|Delay (Variables|Default|GetStopDelay))
      (switch Utilities|FlowControl|Switch|SwitchonETimelineDirection _direction
        (:Forward
          (CallFunction|Rewind))
        (:Backward
          (CallFunction|Forward))))))

(event Custom|Rewind
  (bind (_direction _lerp_alpha) (Timeline|MoveStopTimeline ReverseFromEnd)
    (:Update
      (Transformation|SetRelativeLocation (Variables|Default|GetHitPlayerBox) (Math|Vector|Lerp(Vector) "0, 0, 0" (Variables|Default|GetEndLocation) _lerp_alpha) false))
    (:Finished
      (Utilities|FlowControl|Delay (Variables|Default|GetStopDelay))
      (switch Utilities|FlowControl|Switch|SwitchonETimelineDirection _direction
        (:Forward
          (CallFunction|Rewind))
        (:Backward
          (CallFunction|Forward))))))

(event EventBeginPlay
  (|CallParentFunction))

(event Collision|EventActorBeginOverlap
  (params (OtherActor :type Actor%20Object%20Reference)))

(event EventTick
  (params (DeltaSeconds :type Float%20%28single-precision%29)))

(fn ConstructionScript
  (|CallParentFunction)
  (Transformation|SetActorLocation (Math|Vector|SelectVector (Variables|Default|GetEndLocation) "0, 0, 0" (Variables|Default|GetTestEndLocation)) false))