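; BP_Enemy_Shell is a shell enemy that opens and fires a shot when the player, BP_Dude, enters its detection box.
; On entry it swaps to the open sprite, sets the sprite's yaw from the player-to-shell direction, and after a short delay plays a sound and spawns one BP_Base_Enemy_Shot at ShootArrow's transform.
; On exit it restores the closed sprite and updates the yaw again.
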(event OnComponentBeginOverlap(DetectPlayerBox)
  (params (OtherActor :type Actor%20Object%20Reference) (OtherComp :type Primitive%20Component%20Object%20Reference) (OtherBodyIndex :type Integer) (bFromSweep :type Boolean) (SweepResult :type Hit%20Result%20Structure%20%28by%20ref%29))
  ;[1 1 1] Open shell
  (Utilities|Casting|CastToBP_Dude OtherActor)
  (Rendering|Components|Sprite|SetSprite (Variables|Default|GetShellSprite) "/Game/W995/Sprites/Enemies/shell_02.shell_02")
  (Transformation|SetWorldRotation (Variables|Default|GetShellSprite) (CallFunction|GetFacingRotation) false)
  (Utilities|FlowControl|Delay 0.3)
  (CallFunction|Shoot))

(event OnComponentEndOverlap(DetectPlayerBox)
  (params (OtherActor :type Actor%20Object%20Reference) (OtherComp :type Primitive%20Component%20Object%20Reference) (OtherBodyIndex :type Integer))
  ;[1 1 1] Close shell
  (Utilities|Casting|CastToBP_Dude OtherActor)
  (Rendering|Components|Sprite|SetSprite (Variables|Default|GetShellSprite) "/Game/W995/Sprites/Enemies/shell_01.shell_01")
  (Transformation|SetWorldRotation (Variables|Default|GetShellSprite) (CallFunction|GetFacingRotation) false))

(event Custom|Shoot
  ;[1 1 1] Shoot
  (Audio|PlaySound2D "/Game/W995/Sounds/Enemy_shot_cue.Enemy_shot_cue")
  (CallFunction|Shootat (Transformation|GetWorldTransform (Variables|Default|GetShootArrow))))

(fn ConstructionScript)

(fn GetVectortoPlayer
  (return (Math|Vector|GetForwardVector (Math|Rotator|FindLookatRotation (Transformation|GetActorLocation (Game|GetPlayerCharacter 0)) (Transformation|GetActorLocation)))))

(fn Shootat
  (params (TargetVector :type Transform))
  (Game|SpawnActorfromClass "/Game/W995/Blueprint/Weapons/BP_Base_Enemy_Shot.BP_Base_Enemy_Shot_C" TargetVector false 0 0))

(fn GetFacingRotation
  (return (Class|KismetMathLibrary|MakeRot 0.0 (.Yaw (Class|KismetMathLibrary|BreakRot (Math|Conversions|RotationFromXVector (CallFunction|GetVectortoPlayer)))) 0.0)))