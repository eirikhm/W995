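; Spin shooter enemy that alternates between a closed state and an active, firing state in an endless timed loop started at BeginPlay.
; SwapState toggles IsActive, swaps the flipbook and resizes HitPlayerBox taller when active, then re-calls itself after a per-state delay.
; Each activation calls Shoot, which plays a sound and uses ShootAt to spawn BP_Base_Enemy_Shot at the left and right arrow transforms.
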(event Custom|Shoot
  ;[1 1 1] Shoot
  (Audio|PlaySound2D "/Game/W995/Sounds/shot_connect_Cue.shot_connect_Cue")
  (Utilities|FlowControl|Sequence
    (:then_0
      (CallFunction|Shootat (Transformation|GetWorldTransform (Variables|Default|GetArrowLeft))))
    (:then_1
      (CallFunction|Shootat (Transformation|GetWorldTransform (Variables|Default|GetArrowRight))))))

(event Custom|SwapState
  ;[1 1 1] ChangeState
  (if (Variables|Default|GetisActive)
    (Sprite|SetFlipbook (Variables|Default|GetPaperFlipbook) "/Game/W995/Sprites/Enemies/A_SpinShotClosed.A_SpinShotClosed")
    (Variables|Default|SetisActive false)
    (Components|Box|SetBoxExtent (Variables|Default|GetHitPlayerBox) "8.000000,8.000000,8.000000" true)
    (Utilities|FlowControl|Delay 2.0)
    (else
      (Sprite|SetFlipbook (Variables|Default|GetPaperFlipbook) "/Game/W995/Sprites/Enemies/A_SpinShotActive.A_SpinShotActive")
      (Variables|Default|SetisActive true)
      (Components|Box|SetBoxExtent (Variables|Default|GetHitPlayerBox) "8.000000,8.000000,30.000000" true)
      (CallFunction|Shoot)
      (Utilities|FlowControl|Delay 1.5)))
  (CallFunction|SwapState))

(event EventBeginPlay
  ;[1 1 1] Init
  (CallFunction|SwapState))

(fn ConstructionScript
  (|CallParentFunction))

(fn Shootat
  (params (ShootTransform :type Transform))
  (Game|SpawnActorfromClass "/Game/W995/Blueprint/Weapons/BP_Base_Enemy_Shot.BP_Base_Enemy_Shot_C" ShootTransform false 0 0))