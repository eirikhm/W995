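; Lift that moves its sprite between the local origin and EndLocation along a timeline scaled to TravelTimeInSec.
; On finishing, the timeline waits StopDelay, then runs the opposite way through LiftForward or LiftReturn.
; BP_Dude entering SafetyCollider while the timeline is active calls Play or Reverse on it, based on its playing state.
; The construction script uses TestEndLocation to preview the end position, and BeginPlay clears that flag.
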(event OnComponentBeginOverlap(SafetyCollider)
  (params (OtherActor :type Actor%20Object%20Reference) (OtherComp :type Primitive%20Component%20Object%20Reference) (OtherBodyIndex :type Integer) (bFromSweep :type Boolean) (SweepResult :type Hit%20Result%20Structure%20%28by%20ref%29))
  (bind _lifttimeline (Variables|Default|GetLiftTimeline))
  (Utilities|Casting|CastToBP_Dude OtherActor)
  (if (Components|Activation|IsActive _lifttimeline)
    (if (Audio|Components|Audio|IsPlaying _lifttimeline)
      (bind (_direction _lerpalpha) (Timeline|LiftTimeline Play)
        (:Update
          (Transformation|SetRelativeLocation (Variables|Default|GetLiftSprite) (Math|Vector|Lerp(Vector) "0, 0, 0" (Variables|LiftControls|GetEndLocation) _lerpalpha) false))
        (:Finished
          (Utilities|FlowControl|Delay (Variables|LiftControls|GetStopDelay))
          (switch Utilities|FlowControl|Switch|SwitchonETimelineDirection _direction
            (:Forward
              (CallFunction|LiftReturn))
            (:Backward
              (CallFunction|LiftForward)))))
      (else
        (Timeline|LiftTimeline Reverse)))))

(event Custom|LiftForward
  (bind (_direction _lerpalpha) (Timeline|LiftTimeline PlayFromStart)
    (:Update
      (Transformation|SetRelativeLocation (Variables|Default|GetLiftSprite) (Math|Vector|Lerp(Vector) "0, 0, 0" (Variables|LiftControls|GetEndLocation) _lerpalpha) false))
    (:Finished
      (Utilities|FlowControl|Delay (Variables|LiftControls|GetStopDelay))
      (switch Utilities|FlowControl|Switch|SwitchonETimelineDirection _direction
        (:Forward
          (CallFunction|LiftReturn))
        (:Backward
          (CallFunction|LiftForward))))))

(event Custom|LiftReturn
  (bind (_direction _lerpalpha) (Timeline|LiftTimeline ReverseFromEnd)
    (:Update
      (Transformation|SetRelativeLocation (Variables|Default|GetLiftSprite) (Math|Vector|Lerp(Vector) "0, 0, 0" (Variables|LiftControls|GetEndLocation) _lerpalpha) false))
    (:Finished
      (Utilities|FlowControl|Delay (Variables|LiftControls|GetStopDelay))
      (switch Utilities|FlowControl|Switch|SwitchonETimelineDirection _direction
        (:Forward
          (CallFunction|LiftReturn))
        (:Backward
          (CallFunction|LiftForward))))))

(event EventBeginPlay
  ;[1 1 1] Init
  (Components|Timeline|SetPlayRate (Variables|Default|GetLiftTimeline) (/ 1.0 (Variables|LiftControls|GetTravelTimeInSec)))
  (Variables|LiftControls|SetTestEndLocation false))

(fn ConstructionScript
  (Transformation|SetRelativeLocation (Variables|Default|GetLiftSprite) (Math|Vector|SelectVector (Variables|LiftControls|GetEndLocation) "0, 0, 0" (Variables|LiftControls|GetTestEndLocation)) false))